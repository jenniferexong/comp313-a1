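; Duckling actor with a hunger bar that drains each tick and kills it when depleted, leaving a bone actor behind.
; It chirps and awards the player score on spawn, caching the widget's progress bar and the DuckCharacter.
; Feed refills the bar, enlarges the mesh, lightens its colour via a dynamic material and adds score.
; Feeding works up to three times, and the third removes the hunger widget.
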(event EventBeginPlay
  (Audio|PlaySoundatLocation "/Game/Sounds/chirp.chirp" (Transformation|GetActorLocation) "0, 0, 0" 1.0 1.0 0.0 0 0 0) ; chirp sound
  (bind _ashunger_bar (Utilities|Casting|CastToHungerBar (UserInterface|GetWidget (Variables|Default|GetHungerWidget))))
  (Variables|Default|SetHunger%20Progress (Variables|/Game/UI/HungerBar.HungerBar_C|GetHungerProgress _ashunger_bar))
  (Progress|SetPercent (Variables|/Game/UI/HungerBar.HungerBar_C|GetHungerProgress _ashunger_bar) 1.0)
  (bind _asduck_character (Utilities|Casting|CastToDuckCharacter (Game|GetPlayerCharacter 0)))
  (bind _output_get (Variables|Default|SetPlayer _asduck_character))
  (Class|DuckCharacter|UpdateScore _output_get 10))

(event Collision|EventActorBeginOverlap
  (params (OtherActor :type Actor%20Object%20Reference)))

(event EventTick
  (params (DeltaSeconds :type Float%20%28single-precision%29))
  (CallFunction|Update DeltaSeconds))

(fn ConstructionScript)

(fn Update
  (params (delta :type Float%20%28single-precision%29))
  (bind _hunger_progress (Variables|Default|GetHunger%20Progress))
  (bind _percent (Variables|/Script/UMG.ProgressBar|GetPercent _hunger_progress))
  (if (< _percent 0.0) ; if hunger bar is depleted, kill the duckling
    (CallFunction|Die)
    (else
      (Progress|SetPercent _hunger_progress (- _percent (* (/ delta 5e+01) (Variables|Default|GetHungerSpeed)))))))

(fn Die
  (Game|SpawnActorfromClass "/Game/Scene/Blueprints/Bone_BP.Bone_BP_C" (Math|Conversions|ToTransform(Vector) (Transformation|GetWorldLocation (Variables|Default|GetDuckling))) "AlwaysSpawn" 0 0)
  (Actor|DestroyActor))

(fn Feed
  (bind _duckling (Variables|Default|GetDuckling))
  (if (< (Variables|Default|GetGrowthCount) 3) ; only feed the duckling if it has been \nfed less than 3 times
    (Transformation|SetWorldScale3D _duckling (+ (Transformation|GetWorldScale _duckling) "0.300000,0.300000,0.300000")) ; increase size of duckling
    (CallFunction|LightenColour)
    (Progress|SetPercent (Variables|Default|GetHunger%20Progress) 1.0) ; reset hunger bar
    (Math|Integer|IncrementInt (Variables|Default|GetGrowthCount)
      (:%20%20
        (Class|DuckCharacter|UpdateScore (Variables|Default|GetPlayer) 10) ; add to player score
        (if (== (Variables|Default|GetGrowthCount) 3)
          (Components|DestroyComponent (Variables|Default|GetHungerWidget)))
        (return true)))
    (else
      (return false))))

(fn LightenColour
  (bind _returnvalue (Rendering|Material|CreateDynamicMaterialInstance (Variables|Default|GetDuckling) 0 0 "None" :!class /Script/Engine.PrimitiveComponent)) ; change colour of duckling
  (bind _returnvalue_2 (Rendering|Material|GetVectorParameterValue _returnvalue "Colour" :!class /Script/Engine.MaterialInstanceDynamic))
  (Rendering|Material|SetVectorParameterValue _returnvalue "Colour" (Math|Conversions|ToLinearColor(Vector) (+ (Math|Conversions|ToVector(LinearColor) _returnvalue_2) "0.200000,0.200000,0.200000")) :!class /Script/Engine.MaterialInstanceDynamic))