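; Egg actor that grows over time and hatches into a duckling.
; Tick accumulates time against a random interval chosen once at BeginPlay, advancing the GrowthBar widget's progress bar one fixed step each time it elapses.
; The bar's percent itself holds the growth state; when one further step would reach full, the egg spawns Duckling_BP at the Egg component's transform and destroys itself.
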(event EventBeginPlay
  (Variables|Growth|SetGrowthTime (Math|Random|RandomFloatinRange 1.0 3.0))
  (Variables|Growth|SetTimePassed 0.0)
  (Variables|Growth|SetGrowthStages 10))

(event Collision|EventActorBeginOverlap
  (params (OtherActor :type Actor%20Object%20Reference)))

(event EventTick
  (params (DeltaSeconds :type Float%20%28single-precision%29))
  (CallFunction|IncreaseAge DeltaSeconds)
  (if (> (Variables|Growth|GetTimePassed) (Variables|Growth|GetGrowthTime))
    (Variables|Growth|SetTimePassed 0.0)
    (CallFunction|Grow)))

(fn ConstructionScript)

(fn IncreaseAge
  (params (delta%20time :type Float%20%28single-precision%29))
  (Variables|Growth|SetTimePassed (+ delta%20time (Variables|Growth|GetTimePassed))))

(fn Grow
  (bind _asegg_progress_bar (Utilities|Casting|CastToEggProgressBar (UserInterface|GetWidget (Variables|Default|GetGrowthBar))))
  (Progress|SetPercent (Variables|/Game/UI/EggProgressBar.EggProgressBar_C|GetGrowthProgress _asegg_progress_bar) (+ (Variables|/Script/UMG.ProgressBar|GetPercent (Variables|/Game/UI/EggProgressBar.EggProgressBar_C|GetGrowthProgress _asegg_progress_bar)) (/ 1.0 (Math|Conversions|ToFloat(Integer) (Variables|Growth|GetGrowthStages)))))
  (if (>= (+ (Variables|/Script/UMG.ProgressBar|GetPercent (Variables|/Game/UI/EggProgressBar.EggProgressBar_C|GetGrowthProgress _asegg_progress_bar)) (/ 1.0 (Math|Conversions|ToFloat(Integer) (Variables|Growth|GetGrowthStages)))) 1.0)
    (CallFunction|HatchEgg)))

(fn HatchEgg
  (Game|SpawnActorfromClass "/Game/Scene/Blueprints/Duckling_BP.Duckling_BP_C" (Transformation|GetWorldTransform (Variables|Default|GetEgg)) "AlwaysSpawn" 0 0)
  (Actor|DestroyActor))