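; Player duck character that carries worms to feed ducklings, with HUD, pause and end-screen handling.
; Overlapping a worm sets HasFood and shows the carried worm, and hitting a duckling while holding food calls its Feed, clearing the food on success.
; Left click quacks, dropping any food, playing a sound and reporting an AI noise event.
; Tick polls for game over, which, like Tab pause, shows a UI-only widget and pauses the game.
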(event OnComponentHit(CapsuleComponent)
  (params (HitComponent :type Primitive%20Component%20Object%20Reference) (OtherActor :type Actor%20Object%20Reference) (OtherComp :type Primitive%20Component%20Object%20Reference) (NormalImpulse :type Vector :default "0, 0, 0") (Hit :type Hit%20Result%20Structure%20%28by%20ref%29))
  (CallFunction|AttemptFeed OtherActor))

(event OnComponentBeginOverlap(CapsuleComponent)
  (params (OverlappedComponent :type Primitive%20Component%20Object%20Reference) (OtherActor :type Actor%20Object%20Reference) (OtherComp :type Primitive%20Component%20Object%20Reference) (OtherBodyIndex :type Integer) (bFromSweep :type Boolean) (SweepResult :type Hit%20Result%20Structure%20%28by%20ref%29))
  (if (Utilities|ClassIsChildOf (Utilities|GetClass OtherActor) "/Game/Scene/Blueprints/Worms_BP.Worms_BP_C") ; pick up a worm
    (CallFunction|GetWorm true)))

(event EventBeginPlay
  (bind _returnvalue (UserInterface|CreateWidget "/Game/UI/HUD.HUD_C")) ; Set up score hud
  (bind _output_get (Variables|Default|SetHud%20Reference _returnvalue))
  (UserInterface|Viewport|AddtoViewport _output_get 1)
  (Input|SetInputModeGameOnly (Game|GetPlayerController 0)))

(event Collision|EventActorBeginOverlap
  (params (OtherActor :type Actor%20Object%20Reference)))

(event EventTick
  (params (DeltaSeconds :type Float%20%28single-precision%29))
  (CallFunction|CheckGameOver))

(event Input|KeyboardEvents|Tab
  (params (Key :type Key%20Structure))
  (:Pressed
    (CallFunction|Pause)))

(event Input|MouseEvents|LeftMouseButton
  (params (Key :type Key%20Structure))
  (:Pressed
    (CallFunction|Quack)))

(fn ConstructionScript)

(fn Quack
  (bind _mesh (Variables|Character|GetMesh))
  (bind _returnvalue (Transformation|GetWorldLocation _mesh))
  (CallFunction|GetWorm false) ; drop food
  (Audio|PlaySoundatLocation "/Game/Sounds/quack.quack" _returnvalue "0, 0, 0" 1.0 1.0 0.0 0 0 0)
  (Class|AISenseHearing|ReportNoiseEvent _returnvalue 1.0 self 0.0 "None"))

(fn GetWorm
  (params (Obtain :type Boolean))
  (bind _output_get (Variables|Default|SetHasFood Obtain)) ; pick up food
  (Rendering|SetVisibility (Variables|Default|GetWorm) _output_get false))

(fn CheckGameOver
  (bind _returnvalue (Game|GetPlayerController 0))
  (if (Class|DuckCharacter|IsGameOver) ; switch to end screen
    (Widget|RemovefromParent (Variables|Default|GetHud%20Reference))
    (bind _returnvalue_2 (UserInterface|CreateWidget "/Game/UI/EndGame.EndGame_C"))
    (Variables|/Script/Engine.PlayerController|SetbShowMouseCursor _returnvalue true)
    (Input|SetInputModeUIOnly _returnvalue _returnvalue_2 "DoNotLock")
    (UserInterface|Viewport|AddtoViewport _returnvalue_2 0)
    (Game|SetGamePaused true)))

(fn Pause
  (bind _returnvalue (Game|GetPlayerController 0))
  (Utilities|IsValid (Variables|Default|GetPauseMenu%20reference)
    (:Is%20Valid
      _)
    (:Is%20Not%20Valid
      (bind _returnvalue_2 (UserInterface|CreateWidget "/Game/UI/PauseMenu.PauseMenu_C"))
      (Variables|Default|SetPauseMenu%20reference _returnvalue_2)))
  (Variables|/Script/Engine.PlayerController|SetbShowMouseCursor _returnvalue true)
  (Input|SetInputModeUIOnly _returnvalue (Variables|Default|GetPauseMenu%20reference) "DoNotLock")
  (UserInterface|Viewport|AddtoViewport (Variables|Default|GetPauseMenu%20reference) 0)
  (Game|SetGamePaused true))

(fn AttemptFeed
  (params (actor :type Actor%20Object%20Reference))
  (if (Utilities|ClassIsChildOf (Utilities|GetClass actor) "/Game/Scene/Blueprints/Duckling_BP.Duckling_BP_C")
    (bind _asduckling_bp (Utilities|Casting|CastToDuckling_BP actor)) ; feed duckling on collision, if player is holding food
    (if (Variables|Default|GetHasFood)
      (bind _feedsuccess (Default|Feed _asduckling_bp))
      (if _feedsuccess
        (CallFunction|GetWorm false) ; get rid of food if the duckling was fed
      ))))