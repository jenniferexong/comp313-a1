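; Wolf enemy that stalks an assigned target at a random slow speed and kills eggs or ducklings it collides with.
; Tick-driven logic starts hunts from the spawn point via AI SimpleMoveTo, using boolean state flags.
; Any hearing perception update, meant for quacks, sends it running back to spawn to hunt again.
; After a kill it growls, pauses for the bite animation, flees, and destroys itself at spawn.
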(event OnTargetPerceptionUpdated(Hearing)
  (params (Actor :type Actor%20Object%20Reference) (Stimulus :type AI%20Stimulus%20Structure))
  (CallFunction|Flee))

(event OnComponentHit(CapsuleComponent)
  (params (HitComponent :type Primitive%20Component%20Object%20Reference) (OtherActor :type Actor%20Object%20Reference) (OtherComp :type Primitive%20Component%20Object%20Reference) (NormalImpulse :type Vector :default "0, 0, 0") (Hit :type Hit%20Result%20Structure%20%28by%20ref%29))
  (bind _killed (CallFunction|AttemptKill OtherActor))
  (if _killed
    _))

(event EventBeginPlay
  (bind _asaicontroller (Utilities|Casting|CastToAIController (Pawn|GetController)))
  (Variables|Default|Setcontroller%20ref _asaicontroller)
  (Variables|Default|SetSpawnLocation (Transformation|GetActorLocation))
  (CallFunction|SetWalkSpeed))

(event Collision|EventActorBeginOverlap
  (params (OtherActor :type Actor%20Object%20Reference)))

(event EventTick
  (params (DeltaSeconds :type Float%20%28single-precision%29))
  (CallFunction|Update DeltaSeconds))

(fn ConstructionScript)

(fn AttemptKill
  (params (other%20actor :type Actor%20Object%20Reference))
  (bind _output_get (LocalVariables|Setother other%20actor))
  (if (Utilities|ClassIsChildOf (Utilities|GetClass _output_get) "/Game/Scene/Blueprints/Egg_BP.Egg_BP_C")
    (bind _asegg_bp (Utilities|Casting|CastToEgg_BP (LocalVariables|Getother))) ; kill an egg on collision
    (Default|Die _asegg_bp)
    (Variables|Default|SetIsBiting true :!label _label)
    (Variables|Default|SetKilledTarget true)
    (Audio|PlaySoundatLocation "/Game/Sounds/growl.growl" (Transformation|GetActorLocation) "0, 0, 0" 1.0 1.0 0.0 0 0 0)
    (return true)
    (elif (Utilities|ClassIsChildOf (Utilities|GetClass _output_get) "/Game/Scene/Blueprints/Duckling_BP.Duckling_BP_C") ; kill a duckling on collision
      (bind _asduckling_bp (Utilities|Casting|CastToDuckling_BP (LocalVariables|Getother)))
      (Default|Die _asduckling_bp)
      (goto _label))))

(fn Flee
  (Utilities|FlowControl|Sequence
    (:then_0
      (Variables|Default|SetIsBiting false))
    (:then_1
      (Variables|Default|SetIsRunning true))
    (:then_2
      (Variables|Default|SetIsPreying false))
    (:then_3
      (Variables|/Script/Engine.CharacterMovementComponent|SetMaxWalkSpeed (Variables|Character|GetCharacterMovement) 6e+02))
    (:then_4
      (AI|Navigation|SimpleMovetoLocation (Variables|Default|Getcontroller%20ref) (Variables|Default|GetSpawnLocation)))))

(fn Update
  (params (delta :type Float%20%28single-precision%29))
  (bind _killedtarget (Variables|Default|GetKilledTarget))
  (LocalVariables|SettimeElapsed delta)
  (bind _isatspawn (CallFunction|AtSpawn))
  (if _isatspawn ; check if wolf is at spawn location
    (if _killedtarget ; Check if killed target yet
      (Actor|DestroyActor) ; wolf is not needed anymore
      (else
        (CallFunction|Hunt) ; hunt the prey if it is still alive
      ))
    (elif _killedtarget
      (bind _output_get (Variables|Default|SetKillTimer (+ (Variables|Default|GetKillTimer) (LocalVariables|GettimeElapsed))))
      (if (> _output_get 0.6) ; Check if a certain amount of time has passed after killing,\nbefore running away. This allows time for the bite animation\nto play.
        (CallFunction|Flee)))))

(fn Hunt
  (Utilities|FlowControl|Sequence
    (:then_0
      (Variables|Default|SetIsPreying true))
    (:then_1
      (Variables|Default|SetIsRunning false))
    (:then_2
      (Variables|Default|SetKillTimer 0.0))
    (:then_3
      (CallFunction|SetWalkSpeed))
    (:then_4
      (AI|Navigation|SimpleMovetoLocation (Variables|Default|Getcontroller%20ref) (Variables|Default|GetTarget)))))

(fn SetWalkSpeed
  (Variables|/Script/Engine.CharacterMovementComponent|SetMaxWalkSpeed (Variables|Character|GetCharacterMovement) (Math|Random|RandomFloatinRange 5e+01 2e+02)))

(fn AtSpawn
  (return (Math|Vector|Equal(Vector) (Transformation|GetActorLocation) (Variables|Default|GetSpawnLocation) 5e+01)))