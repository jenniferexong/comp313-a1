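; BP_Duckling is a duckling actor that advances one growth step each time a GrowthTime interval elapses.
; Tick accumulates elapsed time, then resets the timer and calls Grow.
; When Hatched, Grow enlarges the Duckling component by a fixed scale step; otherwise it advances the EggProgressBar in the GrowthBar widget by one fraction of GrowthStages.
; Nothing in this graph sets Hatched.
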(event EventBeginPlay
  (Variables|Growth|SetTimePassed 0.0))

(event Collision|EventActorBeginOverlap
  (params (OtherActor :type Actor%20Object%20Reference)))

(event EventTick
  (params (DeltaSeconds :type Float%20%28single-precision%29))
  (CallFunction|IncreaseAge DeltaSeconds)
  (if (> (Variables|Growth|GetTimePassed) (Variables|Growth|GetGrowthTime))
    (Variables|Growth|SetTimePassed 0.0)
    (CallFunction|Grow)))

(fn ConstructionScript)

(fn Grow
  (bind _duckling (Variables|Default|GetDuckling))
  (if (Variables|Growth|GetHatched)
    (Transformation|SetWorldScale3D _duckling (+ (Transformation|GetWorldScale _duckling) "0.500000,0.500000,0.500000"))
    (else
      (CallFunction|GrowEgg))))

(fn IncreaseAge
  (params (delta%20time :type Float%20%28single-precision%29))
  (Variables|Growth|SetTimePassed (+ delta%20time (Variables|Growth|GetTimePassed))))

(fn GrowEgg
  (bind _asegg_progress_bar (Utilities|Casting|CastToEggProgressBar (UserInterface|GetWidget (Variables|Default|GetGrowthBar))))
  (Progress|SetPercent (Variables|/Game/UI/EggProgressBar.EggProgressBar_C|GetGrowthProgress _asegg_progress_bar) (+ (Variables|/Script/UMG.ProgressBar|GetPercent (Variables|/Game/UI/EggProgressBar.EggProgressBar_C|GetGrowthProgress _asegg_progress_bar)) (/ 1.0 (Math|Conversions|ToFloat(Integer) (Variables|Growth|GetGrowthStages))))))